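; Player-controlled cannon that rotates in yaw and fires a cosmetic explosion effect at its ShootPoint.
; Spin input rotates it immediately and calls MueveEnServidor, named as a server event, which rotates again and drains Salud while turning.
; Shoot passes through DisparoEnServidor to Disparo, which only spawns the emitter.
; Each turning update with Salud below threshold calls ShowAlert, creating a temporary warning widget from the server-named path.
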(event Custom|MueveEnServidor
  (params (Axis :type Float%20%28single-precision%29))
  (CallFunction|Spin Axis)
  (if (!= Axis 0.0)
    (bind _output_get (Variables|Default|SetSalud (- (Variables|Default|GetSalud) (* (Utilities|Time|GetWorldDeltaSeconds) 1e+01))))
    (if (< _output_get 1e+01)
      (CallFunction|ShowAlert))))

(event Custom|Disparo
  (Effects|SpawnEmitterAttached "/Game/StarterContent/Particles/P_Explosion.P_Explosion" (Variables|Default|GetShootPoint) "None" "0, 0, 0" "0, 0, 0" "0.500000,0.500000,0.500000"))

(event Custom|DisparoEnServidor
  (CallFunction|Disparo))

(event Custom|Show%20Alert
  (bind _returnvalue (UserInterface|CreateWidget "/Game/AlertWG.AlertWG_C"))
  (UserInterface|Viewport|AddtoViewport _returnvalue 0)
  (Utilities|FlowControl|Delay 5.0)
  (Widget|RemovefromParent _returnvalue))

(event Input|ActionEvents|InputActionShoot
  (params (Key :type Key%20Structure))
  (:Pressed
    (CallFunction|DisparoEnServidor)))

(event Input|AxisEvents|InputAxisSpin
  (params (AxisValue :type Float%20%28single-precision%29))
  (CallFunction|Spin AxisValue)
  (CallFunction|MueveEnServidor AxisValue))

(fn ConstructionScript)

(fn Spin
  (params (Axis :type Float%20%28single-precision%29))
  (Transformation|AddActorLocalRotation (Math|Rotator|MakeRotator 0.0 0.0 (* (* Axis (Variables|Default|GetRotationSpeed)) (Utilities|Time|GetWorldDeltaSeconds))) false false)
  (return))